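; BP_Counting is an actor that displays a single-digit counter on a text render component.
; Each SwitchTrigger event increments Count, wraps it to zero once it passes nine, then writes the value to the text.
; The three steps are split into small functions called in sequence from the event graph.
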(event EventSwitchTrigger
  (CallFunction|DoCountUp)
  (CallFunction|Over9Count0)
  (CallFunction|ShowCount))

(fn ConstructionScript)

(fn DoCountUp
  (Variables|Default|SetCount (+ (Variables|Default|GetCount) 1)))

(fn Over9Count0
  (if (> (Variables|Default|GetCount) 9)
    (Variables|Default|SetCount 0)))

(fn ShowCount
  (Rendering|Components|TextRender|SetText (Variables|Default|GetTextRender) (Utilities|Text|ToText(String) (Utilities|String|ToString(Integer) (Variables|Default|GetCount)))))