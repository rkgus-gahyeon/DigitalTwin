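; BP_MoveRect is an actor that moves its Cube in axis-aligned steps on the X/Z plane, toggled by a Switch.
; BeginPlay binds to the Switch's toggle dispatcher, and EventSwitchToggle sets IsPlay to gate Tick.
; Tick switches on MoveType, adding a fixed per-frame step to the relative location without delta-time scaling.
; Only Right-to-Up transitions are implemented; the Left check and the four Move functions are empty.
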(event EventTick
  (params (DeltaSeconds :type Float%20%28single-precision%29))
  (if (Variables|Default|GetIsPlay)
    (switch Utilities|FlowControl|Switch|SwitchonEN_MoveType (Variables|Default|GetMoveType)
      (:NewEnumerator0
        (Variables|Default|SetPosX (+ (Variables|Default|GetPosX) 1e+01))
        (Transformation|SetRelativeLocation (Variables|Default|GetCube) (Math|Vector|MakeVector (Variables|Default|GetPosX) 0.0 (Variables|Default|GetPosZ)) false false)
        (if (> (Variables|Default|GetPosX) 0.0)
          (Variables|Default|SetMoveType "NewEnumerator1")))
      (:NewEnumerator1
        (Variables|Default|SetPosZ (+ (Variables|Default|GetPosZ) 1e+01))
        (Transformation|SetRelativeLocation (Variables|Default|GetCube) (Math|Vector|MakeVector (Variables|Default|GetPosX) 0.0 (Variables|Default|GetPosZ)) false false))
      (:NewEnumerator2
        (Variables|Default|SetPosX (+ (Variables|Default|GetPosX) -1e+01))
        (Transformation|SetRelativeLocation (Variables|Default|GetCube) (Math|Vector|MakeVector (Variables|Default|GetPosX) 0.0 (Variables|Default|GetPosZ)) false false)
        (if (< (Variables|Default|GetPosX) 0.0)
          _))
      (:NewEnumerator3
        (Variables|Default|SetPosZ (+ (Variables|Default|GetPosZ) -1e+01))
        (Transformation|SetRelativeLocation (Variables|Default|GetCube) (Math|Vector|MakeVector (Variables|Default|GetPosX) 0.0 (Variables|Default|GetPosZ)) false false)))))

(event EventBeginPlay
  (EventDispatchers|BindEventtoEventDispatcherToggle (Variables|Default|GetSwitch) (EventDispatchers|CreateEvent :!event EventSwitchToggle)))

(fn ConstructionScript)

(fn MoveRight)

(fn MoveUp)

(fn MoveLeft)

(fn MoveDown)

(fn EventSwitchToggle
  (params (Toggle :type Boolean))
  (Variables|Default|SetIsPlay Toggle))